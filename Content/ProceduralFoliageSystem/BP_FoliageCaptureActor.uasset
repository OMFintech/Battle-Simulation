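; Capture actor for procedural foliage that builds foliage transforms over a Cesium 3D Tileset, first run after a short delay on BeginPlay.
; Orthographic imagery, normals and depth scene captures render only that tileset across CaptureWidth.
; On update, it runs the parent logic, captures, and advances Niagara one tick, with next-tick delays between stages.
; BuildFoliageTransforms then receives the classification and normal render targets plus the capture area's world bounds.
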(event Custom|Debug
  (Class|FoliageCaptureActor|OnUpdate (Transformation|GetActorLocation)))

(event EventBeginPlay
  ;[1 1 1] activate components
  (Components|Activation|Activate (Variables|Default|GetImagery) false)
  (Components|Activation|Activate (Variables|Default|GetNiagara) false)
  ;[1 1 1] Initally spawn foliage after 2 seconds
  (Utilities|FlowControl|Delay 2.0)
  (Class|FoliageCaptureActor|OnUpdate (Transformation|GetActorLocation)))

(event Collision|EventActorBeginOverlap
  (params (OtherActor :type Actor%20Object%20Reference)))

(event EventTick
  (params (DeltaSeconds :type Float%20%28single-precision%29)))

(event EventOnUpdate
  (params (NewLocation :type Vector%20%28by%20ref%29 :default "0, 0, 0"))
  (bind _returnvalue (Transformation|GetActorTransform))
  (bind _capturewidth (Variables|Default|GetCaptureWidth))
  (bind _returnvalue_2 (* _capturewidth 0.5))
  (bind _returnvalue_3 (* _capturewidth -0.5))
  (|CallParentFunction NewLocation)
  (Utilities|FlowControl|DelayUntilNextTick)
  (Rendering|SceneCapture|CaptureScene (Variables|Default|GetImagery) :!class /Script/Engine.SceneCaptureComponent2D)
  (Class|NiagaraComponent|AdvanceSimulation (Variables|Default|GetNiagara) 1 (Utilities|Time|GetWorldDeltaSeconds))
  (Utilities|FlowControl|DelayUntilNextTick)
  (Class|FoliageCaptureActor|BuildFoliageTransforms "/Game/RenderTargets/RT_Classifications.RT_Classifications" "/Game/RenderTargets/RT_Normals.RT_Normals" (Math|Box|MakeBox (Math|Transform|TransformLocation _returnvalue (Math|Vector|MakeVector _returnvalue_3 _returnvalue_3 0.0)) (Math|Transform|TransformLocation _returnvalue (Math|Vector|MakeVector _returnvalue_2 _returnvalue_2 0.0)))))

(fn ConstructionScript
  (bind _imagery (Variables|Default|GetImagery))
  (bind _capturewidth (Variables|Default|GetCaptureWidth))
  (bind _normals (Variables|Default|GetNormals))
  (bind _depth (Variables|Default|GetDepth))
  (bind _relevant_cesium3d_tileset (Variables|Default|GetRelevant%20Cesium3D%20Tileset))
  (bind _array (Utilities|Array|MakeArray _relevant_cesium3d_tileset))
  (Variables|/Script/Engine.SceneCaptureComponent2D|SetOrthoWidth _imagery _capturewidth)
  (Variables|/Script/Engine.SceneCaptureComponent2D|SetOrthoWidth _normals _capturewidth)
  (Variables|/Script/Engine.SceneCaptureComponent2D|SetOrthoWidth _depth _capturewidth)
  (Variables|/Script/Engine.SceneCaptureComponent|SetPrimitiveRenderMode _imagery "PRM_UseShowOnlyList")
  (Variables|/Script/Engine.SceneCaptureComponent|SetPrimitiveRenderMode _normals "PRM_UseShowOnlyList")
  (Variables|/Script/Engine.SceneCaptureComponent|SetPrimitiveRenderMode _depth "PRM_UseShowOnlyList")
  (Variables|/Script/Engine.SceneCaptureComponent|SetShowOnlyActors _imagery _array)
  (Variables|/Script/Engine.SceneCaptureComponent|SetShowOnlyActors _normals _array)
  (Variables|/Script/Engine.SceneCaptureComponent|SetShowOnlyActors _depth _array)
  (Class|SceneCaptureComponent|SetCaptureSortPriority (Variables|Default|GetNormals) 900000000))